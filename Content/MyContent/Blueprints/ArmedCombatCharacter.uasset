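; Armed character Blueprint that carries primary, secondary and sidearm guns as child actors and handles switching, aiming, shooting and reloading.
; EquipGun hides all three guns, then shows the selected one and snaps it to the mesh's WeaponSocket, starting with the primary.
; Shooting calls go to EquippedGun, set only from the primary in construction, and reload also targets the primary.
; Aim input sets IsAiming on the character and its AnimBP.
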(event Custom|StartShooting
  (Variables|Default|SetIsShooting true)
  (Default|StartShooting (Variables|Default|GetEquippedGun))
  (Animation|Montage|PlayMontage (Variables|Character|GetMesh) 0
    (:then
      (Development|PrintString "Shooting"))))

(event Custom|StopShooting
  (Variables|Default|SetIsShooting false)
  (Default|StopShooting (Variables|Default|GetEquippedGun)))

(event Custom|Threatened
  (Variables|Default|SetIsInDanger true)
  (Development|PrintString "Threatened!!!"))

(event Custom|SelectPrimaryWeapon
  (Variables|Default|SetCurrentlyEquipped 0)
  (CallFunction|EquipGun))

(event EventBeginPlay
  (CallFunction|SelectPrimaryWeapon))

(event Input|ActionEvents|InputActionPrimaryWeapon
  (params (Key :type Key%20Structure :default "None"))
  (:Pressed
    (Variables|Default|SetCurrentlyEquipped 0)
    (CallFunction|EquipGun)))

(event Input|ActionEvents|InputActionSecondaryWeapon
  (params (Key :type Key%20Structure :default "None"))
  (:Pressed
    (Variables|Default|SetCurrentlyEquipped 1)
    (CallFunction|EquipGun)))

(event Input|ActionEvents|InputActionSideArm
  (params (Key :type Key%20Structure :default "None"))
  (:Pressed
    (Variables|Default|SetCurrentlyEquipped 2)
    (CallFunction|EquipGun)))

(event Input|ActionEvents|InputActionReload
  (params (Key :type Key%20Structure :default "None"))
  (:Pressed
    (bind _asgun_master_bp (Utilities|Casting|CastToGunMaster_BP (Variables|/Script/Engine.ChildActorComponent|GetChildActor (Variables|Default|GetPrimaryGun))))
    (Default|Reload _asgun_master_bp)))

(event Input|ActionEvents|InputActionAim
  (params (Key :type Key%20Structure :default "None"))
  (bind _mesh (Variables|Character|GetMesh))
  (bind _returnvalue (Components|SkeletalMesh|GetAnimInstance _mesh))
  (:Pressed
    (Variables|Default|SetIsAiming true)
    (bind _asarmed_combat_character_anim_bp (Utilities|Casting|CastToArmedCombatCharacter_AnimBP _returnvalue))
    (Variables|/Game/MyContent/Blueprints/ArmedCombatCharacter_AnimBP.ArmedCombatCharacter_AnimBP_C|SetIsAiming _asarmed_combat_character_anim_bp true))
  (:Released
    (Variables|Default|SetIsAiming false)
    (bind _asarmed_combat_character_anim_bp_2 (Utilities|Casting|CastToArmedCombatCharacter_AnimBP _returnvalue))
    (Variables|/Game/MyContent/Blueprints/ArmedCombatCharacter_AnimBP.ArmedCombatCharacter_AnimBP_C|SetIsAiming _asarmed_combat_character_anim_bp_2 false)))

(fn ConstructionScript
  (|CallParentFunction)
  (bind _asgun_master_bp (Utilities|Casting|CastToGunMaster_BP (Variables|/Script/Engine.ChildActorComponent|GetChildActor (Variables|Default|GetPrimaryGun))))
  (Variables|Default|SetEquippedGun _asgun_master_bp)
  (Transformation|AttachComponentToComponent (Variables|Default|GetPrimaryGun) (Variables|Character|GetMesh) "WeaponSocket" "SnapToTarget" "SnapToTarget" "SnapToTarget" true))

(fn EquipGun
  (bind _primarygun (Variables|Default|GetPrimaryGun))
  (bind _secondarygun (Variables|Default|GetSecondaryGun))
  (bind _sidearmgun (Variables|Default|GetSideArmGun))
  (bind _currentlyequipped (Variables|Default|GetCurrentlyEquipped))
  (bind _array (Utilities|Array|MakeArray _primarygun _secondarygun _sidearmgun))
  (bind _output (Utilities|Array|Get(acopy) _array _currentlyequipped))
  (for _array_element _array
    (Rendering|SetVisibility _array_element false false))
  (Rendering|SetVisibility _output true false)
  (Transformation|AttachComponentToComponent _output (Variables|Character|GetMesh) "WeaponSocket" "SnapToTarget" "SnapToTarget" "SnapToTarget" true))

(fn SpawnProjectile
  (bind _returnvalue (Game|SpawnActorfromClass "/Game/FirstPersonBP/Blueprints/FirstPersonProjectile.FirstPersonProjectile_C" (Transformation|GetSocketTransform (Variables|Character|GetMesh) "WeaponSocket" "RTS_World") "AlwaysSpawn" self 0))
  (return (Utilities|IsValid _returnvalue)))