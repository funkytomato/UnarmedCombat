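; Parkour character Blueprint that vaults, gets up on or climbs walls ahead when Vault is pressed.
; VaultOrClimb line-traces the wall face, top and far side to classify height and thickness, choosing the move; climbs over thin walls add a jump down.
; Moves snap the actor, disable capsule collision and use Flying during root-motion montages, then restore Walking.
; An upper forward trace blocks climbing by clearing CanClimb, which is never reset here.
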(event EventBeginPlay
  (|CallParentFunction) ; This node is disabled and will not be called.\nDrag off pins to build functionality.
)

(event Input|ActionEvents|InputActionVault
  (params (Key :type Key%20Structure :default "None"))
  ;[1 1 1] vault/Climb
  (:Pressed
    (Utilities|VaultorClimb)))

(fn ConstructionScript
  (|CallParentFunction))