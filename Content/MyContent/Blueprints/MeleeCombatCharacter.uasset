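; Melee combat character that attacks with a sword, damages NPC-tagged actors and loses health when hit.
; Construction snaps the weapon component to the mesh's sword socket, and BeginPlay caches the anim instance and weapon child actor.
; Attack input sets IsAttacking and plays a heavy combo montage.
; MeleeCollision overlaps apply point damage without checking IsAttacking, while incoming damage feeds DecreaseHealth.
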(event OnComponentHit(Mesh)
  (params (HitComponent :type Primitive%20Component%20Object%20Reference) (OtherActor :type Actor%20Object%20Reference) (OtherComp :type Primitive%20Component%20Object%20Reference) (NormalImpulse :type Vector :default "0, 0, 0") (Hit :type Hit%20Result%20Structure%20%28by%20ref%29)))

(event OnComponentBeginOverlap(Mesh)
  (params (OverlappedComponent :type Primitive%20Component%20Object%20Reference) (OtherActor :type Actor%20Object%20Reference) (OtherComp :type Primitive%20Component%20Object%20Reference) (OtherBodyIndex :type Integer) (bFromSweep :type Boolean) (SweepResult :type Hit%20Result%20Structure%20%28by%20ref%29)))

(event OnComponentBeginOverlap(MeleeCollision)
  (params (OverlappedComponent :type Primitive%20Component%20Object%20Reference) (OtherActor :type Actor%20Object%20Reference) (OtherComp :type Primitive%20Component%20Object%20Reference) (OtherBodyIndex :type Integer) (bFromSweep :type Boolean) (SweepResult :type Hit%20Result%20Structure%20%28by%20ref%29))
  (if (Actor|ActorHasTag OtherActor "NPC")
    (if (!= OtherActor self)
      (Game|Damage|ApplyPointDamage OtherActor 1.0 (.ImpactNormal (Collision|BreakHitResult SweepResult)) SweepResult 0 self "/Script/Engine.DamageType"))))

(event OnComponentHit(CapsuleComponent)
  (params (HitComponent :type Primitive%20Component%20Object%20Reference) (OtherActor :type Actor%20Object%20Reference) (OtherComp :type Primitive%20Component%20Object%20Reference) (NormalImpulse :type Vector :default "0, 0, 0") (Hit :type Hit%20Result%20Structure%20%28by%20ref%29)))

(event OnComponentBeginOverlap(CapsuleComponent)
  (params (OverlappedComponent :type Primitive%20Component%20Object%20Reference) (OtherActor :type Actor%20Object%20Reference) (OtherComp :type Primitive%20Component%20Object%20Reference) (OtherBodyIndex :type Integer) (bFromSweep :type Boolean) (SweepResult :type Hit%20Result%20Structure%20%28by%20ref%29)))

(event EventBeginPlay
  (|CallParentFunction)
  (bind _asmelee_combat_character_anim_bp (Utilities|Casting|CastToMeleeCombatCharacter_AnimBP (Components|SkeletalMesh|GetAnimInstance (Variables|Character|GetMesh))))
  (Variables|Default|SetAnimInstance _asmelee_combat_character_anim_bp)
  (bind _asmelee_master_bp (Utilities|Casting|CastToMeleeMaster_BP (Variables|/Script/Engine.ChildActorComponent|GetChildActor (Variables|Default|GetWeaponComponent))))
  (Variables|Default|SetCurrentMelee _asmelee_master_bp))

(event Game|Damage|EventAnyDamage
  (params (Damage :type Float%20%28single-precision%29) (DamageType :type Damage%20Type%20Object%20Reference) (InstigatedBy :type Controller%20Object%20Reference) (DamageCauser :type Actor%20Object%20Reference))
  (CallFunction|DecreaseHealth Damage))

(event Input|ActionEvents|InputActionAttack
  (params (Key :type Key%20Structure :default "None"))
  (:Pressed
    (Variables|Default|SetIsAttacking? true)
    (Animation|Montage|MontagePlay (Components|SkeletalMesh|GetAnimInstance (Variables|Character|GetMesh)) "/Game/MyContent/Animations/SwordAndShield/Sowrd_Attack_Combo_CL_Heavy_Montage.Sowrd_Attack_Combo_CL_Heavy_Montage" 1.0 "MontageLength" 0.0 true))
  (:Released
    (Variables|Default|SetIsAttacking? false)))

(fn ConstructionScript
  (|CallParentFunction)
  (Transformation|AttachComponentToComponent (Variables|Default|GetWeaponComponent) (Variables|Character|GetMesh) "SwordSocket" "SnapToTarget" "SnapToTarget" "SnapToTarget" true))