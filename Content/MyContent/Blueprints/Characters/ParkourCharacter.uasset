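; Player character Blueprint for parkour, with toggle crouch, montage-driven sliding, and a single input for vaulting or climbing obstacles.
; VaultOrClimb uses line traces to measure wall height and thickness and check upper clearance, selecting vault, get-up, climb, or climb then jump down.
; Moves align the actor to the wall and play montages, mostly root-motion, while capsule collision is off and movement is Flying, then restore Walking.
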(event EventBeginPlay
  (|CallParentFunction) ; This node is disabled and will not be called.\nDrag off pins to build functionality.
)

(event Input|ActionEvents|InputActionVault
  (params (Key :type Key%20Structure :default "None"))
  ;[1 1 1] vault/Climb
  (:Pressed
    (Utilities|VaultorClimb)))

(event Input|ActionEvents|InputActionSlide
  (params (Key :type Key%20Structure :default "None"))
  ;[1 1 1] Sliding
  (:Pressed
    (Pawn|Components|CharacterMovement|SetMovementMode (Variables|Character|GetCharacterMovement) "MOVE_Flying" 0)
    (Collision|SetCollisionEnabled (Variables|Default|GetCapsuleComponent) "NoCollision")
    (bind _returnvalue (Animation|PlayAnimMontage (Game|GetPlayerCharacter 0) "/Game/MyContent/Animations/Parkour/Slide_Montage.Slide_Montage" 1.0 "None"))
    (Utilities|FlowControl|Delay _returnvalue)
    (Collision|SetCollisionEnabled (Variables|Default|GetCapsuleComponent) "QueryAndPhysics")
    (Pawn|Components|CharacterMovement|SetMovementMode (Variables|Character|GetCharacterMovement) "MOVE_Walking" 0)))

(event Input|ActionEvents|InputActionCrouch
  (params (Key :type Key%20Structure :default "None"))
  ;[1 1 1] Crouch
  (:Pressed
    (Utilities|FlowControl|FlipFlop
      (:A
        (Character|Crouch)
        (Variables|Default|SetIsCrouching? true))
      (:B
        (Character|UnCrouch)
        (Variables|Default|SetIsCrouching? false)))))

(fn ConstructionScript
  (|CallParentFunction))