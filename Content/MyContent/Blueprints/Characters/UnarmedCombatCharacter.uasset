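; Player-controllable unarmed fighter character with punches, kicks, blocks, dodges and a stealth takedown.
; Punch plays a random montage with movement locked, while other combat inputs only set held-state booleans; overlapping a punching fighter plays a groan.
; TakedownArea overlaps enable takedowns, which line-trace a target, snap behind it, play paired montages with the camera on the spine, then destroy the victim.
; Hit-reaction and damage logic is present but unconnected.
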(event OnComponentBeginOverlap(TakedownArea)
  (params (OverlappedComponent :type Primitive%20Component%20Object%20Reference) (OtherActor :type Actor%20Object%20Reference) (OtherComp :type Primitive%20Component%20Object%20Reference) (OtherBodyIndex :type Integer) (bFromSweep :type Boolean) (SweepResult :type Hit%20Result%20Structure%20%28by%20ref%29))
  (bind _asunarmed_combat_character (Utilities|Casting|CastToUnarmedCombatCharacter OtherActor))
  (Variables|UnarmedCombatCharacter_C|SetCanTakeDown? _asunarmed_combat_character true))

(event OnComponentEndOverlap(TakedownArea)
  (params (OverlappedComponent :type Primitive%20Component%20Object%20Reference) (OtherActor :type Actor%20Object%20Reference) (OtherComp :type Primitive%20Component%20Object%20Reference) (OtherBodyIndex :type Integer))
  (bind _asunarmed_combat_character (Utilities|Casting|CastToUnarmedCombatCharacter OtherActor))
  (Variables|UnarmedCombatCharacter_C|SetCanTakeDown? _asunarmed_combat_character false))

(event Custom|TakedownSequence
  (Pawn|Components|CharacterMovement|DisableMovement (Variables|Character|GetCharacterMovement))
  (Collision|SetActorEnableCollision false)
  (Animation|PlayAnimMontage "/Game/MyContent/Animations/Takedown/AssassinationEnemy_Montage.AssassinationEnemy_Montage" 1.0 "None")
  (Utilities|FlowControl|Delay 1e+01)
  (Actor|DestroyActor))

(event EventBeginPlay
  (|CallParentFunction))

(event Collision|EventActorBeginOverlap
  (params (OtherActor :type Actor%20Object%20Reference))
  (bind _asunarmed_combat_character (Utilities|Casting|CastToUnarmedCombatCharacter OtherActor))
  (if (Variables|UnarmedCombatCharacter_C|GetisPunching? _asunarmed_combat_character)
    (Audio|PlaySoundatLocation "/Game/MyContent/Audio/GroanImpact_Cue.GroanImpact_Cue" (Transformation|GetActorLocation) "0, 0, 0" 1.0 1.0 0.0 0 0 0)))

(event Input|ActionEvents|InputActionLeftJab
  (params (Key :type Key%20Structure))
  (:Pressed
    (Variables|Default|SetIsLeftJab true))
  (:Released
    (Variables|Default|SetIsLeftJab false)))

(event Input|ActionEvents|InputActionRightJab
  (params (Key :type Key%20Structure))
  (:Pressed
    (Variables|Default|SetIsRightJab true))
  (:Released
    (Variables|Default|SetIsRightJab false)))

(event Input|ActionEvents|InputActionDuckLeft
  (params (Key :type Key%20Structure))
  (:Pressed
    (Variables|Default|SetIsDuckingLeft true))
  (:Released
    (Variables|Default|SetIsDuckingLeft false)))

(event Input|ActionEvents|InputActionDuckRight
  (params (Key :type Key%20Structure))
  (:Pressed
    (Variables|Default|SetIsDuckingRight true))
  (:Released
    (Variables|Default|SetIsDuckingRight false)))

(event Input|ActionEvents|InputActionLeftLowKick
  (params (Key :type Key%20Structure))
  (:Pressed
    (Variables|Default|SetIsLeftLowKick true))
  (:Released
    (Variables|Default|SetIsLeftLowKick false)))

(event Input|ActionEvents|InputActionRightLowKick
  (params (Key :type Key%20Structure))
  (:Pressed
    (Variables|Default|SetIsRightLowKick true))
  (:Released
    (Variables|Default|SetIsRightLowKick false)))

(event Input|ActionEvents|InputActionPunch
  (params (Key :type Key%20Structure))
  (bind _charactermovement (Variables|Character|GetCharacterMovement))
  (:Pressed
    (if (not (AI|Components|NavMovement|IsFalling (Variables|Character|GetCharacterMovement)))
      (if (not (Variables|Default|GetisPunching?))
        (Variables|Default|SetisPunching? true)
        (Pawn|Components|CharacterMovement|DisableMovement _charactermovement)
        (bind _returnvalue (Animation|PlayAnimMontage (Utilities|Array|Get(acopy) (Variables|Default|GetPunchAnimMontage) (Math|Random|RandomIntegerinRange 0 4)) 1.0 "None"))
        (Utilities|FlowControl|Delay _returnvalue)
        (Pawn|Components|CharacterMovement|SetMovementMode _charactermovement "MOVE_Walking" 0)
        (Variables|Default|SetisPunching? false)))))

(event Input|ActionEvents|InputActionTakedown
  (params (Key :type Key%20Structure))
  (bind _returnvalue (Transformation|GetActorLocation))
  (:Pressed
    (if (Variables|Default|GetCanTakeDown?)
      (bind (_outhit _returnvalue_2) (Collision|LineTraceByChannel _returnvalue (+ _returnvalue (* (Transformation|GetActorForwardVector) 2.5e+02)) "TraceTypeQuery1" false 0 "None"))
      (if _returnvalue_2
        (bind _asunarmed_combat_character (Utilities|Casting|CastToUnarmedCombatCharacter (.HitActor (Collision|BreakHitResult _outhit))))
        (Variables|Default|SetTakedownTarget _asunarmed_combat_character)
        (Transformation|AttachComponentToComponent (Variables|Default|GetCameraBoom) (Variables|Character|GetMesh) "spine_02" "SnapToTarget" "SnapToTarget" "SnapToTarget" true)
        (Pawn|Components|CharacterMovement|DisableMovement (Variables|Character|GetCharacterMovement))
        (Variables|Default|SetCanTakeDown? false)
        (Transformation|SetActorTransform (Math|Transform|MakeTransform (+ (.location (Transformation|GetActorTransform (Variables|Default|GetTakedownTarget))) (* (Transformation|GetActorForwardVector (Variables|Default|GetTakedownTarget)) -175.0)) (.rotation (Transformation|GetActorTransform (Variables|Default|GetTakedownTarget))) "1,1,1"))
        (bind _returnvalue_3 (Animation|PlayAnimMontage "/Game/MyContent/Animations/Takedown/AssassinationAttacker_Montage.AssassinationAttacker_Montage" 1.0 "None"))
        (CallFunction|TakedownSequence (Variables|Default|GetTakedownTarget))
        (Utilities|FlowControl|Delay (+ _returnvalue_3 0.025))
        (Transformation|SetActorLocation (+ (Transformation|GetActorLocation) (* (Transformation|GetActorForwardVector) 175.0)) false false)
        (Pawn|Components|CharacterMovement|SetMovementMode (Variables|Character|GetCharacterMovement) "MOVE_Walking" 0)
        (Transformation|AttachComponentToComponent (Variables|Default|GetCameraBoom) (Variables|Default|GetCapsuleComponent) "None" "KeepRelative" "KeepRelative" "KeepRelative" true)))))

(event Input|ActionEvents|InputActionLeftHook
  (params (Key :type Key%20Structure))
  (:Pressed
    (Variables|Default|SetIsLeftHook true))
  (:Released
    (Variables|Default|SetIsLeftHook false)))

(event Input|ActionEvents|InputActionRightHook
  (params (Key :type Key%20Structure))
  (:Pressed
    (Variables|Default|SetIsRightHook true))
  (:Released
    (Variables|Default|SetIsRightHook false)))

(event Input|ActionEvents|InputActionBlock
  (params (Key :type Key%20Structure))
  (:Pressed
    (Variables|Default|SetIsBlocking true))
  (:Released
    (Variables|Default|SetIsBlocking false)))

(event Input|ActionEvents|InputActionLeftUpperCut
  (params (Key :type Key%20Structure))
  (:Pressed
    (Variables|Default|SetIsLeftUpperCut true))
  (:Released
    (Variables|Default|SetIsLeftUpperCut false)))

(event Input|ActionEvents|InputActionRightUpperCut
  (params (Key :type Key%20Structure))
  (:Pressed
    (Variables|Default|SetIsRightUpperCut true))
  (:Released
    (Variables|Default|SetIsRightUpperCut false)))

(event Input|ActionEvents|InputActionDodgeLeft
  (params (Key :type Key%20Structure))
  (:Pressed
    (Variables|Default|SetIsDodgeLeft true))
  (:Released
    (Variables|Default|SetIsDodgeLeft false)))

(event Input|ActionEvents|InputActionDodgeRight
  (params (Key :type Key%20Structure))
  (:Pressed
    (Variables|Default|SetIsDodgeRight true))
  (:Released
    (Variables|Default|SetIsDodgeRight false)))

(event Input|ActionEvents|InputActionDuck
  (params (Key :type Key%20Structure))
  (:Pressed
    (Variables|Default|SetIsDucking true))
  (:Released
    (Variables|Default|SetIsDucking false)))

(fn ConstructionScript
  (|CallParentFunction))