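; Character Blueprint for melee combat, with a punch input and damage taken from other punching characters.
; Pressing Punch on the ground plays a random punch montage, setting IsPunching and disabling movement until the montage's length elapses.
; When a CloseCombatCharacter that is punching begins overlapping it, this character plays a groan impact sound and a random hit montage, then loses health after that montage's delay.
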(event EventBeginPlay
  ;[1 1 1] BeginPlay
  (|CallParentFunction))

(event Collision|EventActorBeginOverlap
  (params (OtherActor :type Actor%20Object%20Reference))
  ;[1 1 1] Hit
  (bind _asclose_combat_character (Utilities|Casting|CastToCloseCombatCharacter OtherActor))
  (if (Variables|CloseCombatCharacter_C|GetisPunching? _asclose_combat_character)
    (Audio|PlaySoundatLocation "/Game/MyContent/Audio/GroanImpact_Cue.GroanImpact_Cue" (Transformation|GetActorLocation) "0, 0, 0" 1.0 1.0 0.0 0 0 0)
    (bind _returnvalue (Animation|PlayAnimMontage (Utilities|Array|Get(acopy) (Variables|Default|GetHitAnimMontage) (Math|Random|RandomIntegerinRange 0 8)) 1.0 "None"))
    (Utilities|FlowControl|Delay _returnvalue)
    (CallFunction|DecreaseHealth 5.0)))

(event Input|ActionEvents|InputActionPunch
  (params (Key :type Key%20Structure :default "None"))
  (bind _charactermovement (Variables|Character|GetCharacterMovement))
  ;[1 1 1] Punch
  (:Pressed
    (if (not (AI|Components|NavMovement|IsFalling (Variables|Character|GetCharacterMovement)))
      (if (not (Variables|Default|GetisPunching?))
        (Variables|Default|SetisPunching? true)
        (Pawn|Components|CharacterMovement|DisableMovement _charactermovement)
        (bind _returnvalue (Animation|PlayAnimMontage (Utilities|Array|Get(acopy) (Variables|Default|GetPunchAnimMontage) (Math|Random|RandomIntegerinRange 0 4)) 1.0 "None"))
        (Utilities|FlowControl|Delay _returnvalue)
        (Pawn|Components|CharacterMovement|SetMovementMode _charactermovement "MOVE_Walking" 0)
        (Variables|Default|SetisPunching? false)))))

(fn ConstructionScript
  (|CallParentFunction))