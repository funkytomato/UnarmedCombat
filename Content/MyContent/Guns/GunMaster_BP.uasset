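; Base gun Blueprint that operates as a child actor of an ArmedCombatCharacter, attaching its mesh to the Arms grip socket.
; FireProjectile either camera-traces to push physics objects (hitscan) or spawns a projectile along camera aim.
; Only the projectile path consumes ammo and runs ThreatTrace, a sphere trace that calls Threatened on a hit ArmedCombatCharacter.
; Start/StopShooting only toggle IsFiring, while Reload refills the clip from reserve ammo.
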(event Custom|StartShooting
  (Variables|Default|SetIsFiring true))

(event Custom|StopShooting
  (Variables|Default|SetIsFiring false))

(fn ConstructionScript
  (Transformation|AttachComponentToComponent (Variables|Default|GetGunMesh) (Variables|Default|GetArms) "GripPoint" "SnapToTarget" "SnapToTarget" "SnapToTarget" true))

(fn FireProjectile
  (bind _asarmed_combat_character (Utilities|Casting|CastToArmedCombatCharacter (Actor|GetParentActor)))
  (Variables|Default|SetGunOwner _asarmed_combat_character)
  (if (Variables|Default|GetIsHitScan)
    (if (> (Variables|Default|GetAmmoCount) 0)
      (if true
        (Variables|Default|SetGunDirection (Math|Vector|GetForwardVector (Transformation|GetWorldRotation (Variables|/Game/MyContent/Blueprints/Characters/MasterCharacter.MasterCharacter_C|GetFollowCamera (Variables|Default|GetGunOwner)))))
        (bind _outhit (Collision|LineTraceByChannel (Transformation|GetWorldLocation (Variables|/Game/MyContent/Blueprints/Characters/MasterCharacter.MasterCharacter_C|GetFollowCamera (Variables|Default|GetGunOwner))) (+ (Transformation|GetWorldLocation (Variables|/Game/MyContent/Blueprints/Characters/MasterCharacter.MasterCharacter_C|GetFollowCamera (Variables|Default|GetGunOwner))) (* (Math|Vector|GetForwardVector (Transformation|GetWorldRotation (Variables|/Game/MyContent/Blueprints/Characters/MasterCharacter.MasterCharacter_C|GetFollowCamera (Variables|Default|GetGunOwner)))) 2e+03)) "TraceTypeQuery1" false 0 "ForDuration"))
        (if (.bBlockingHit (Collision|BreakHitResult _outhit))
          (if (Physics|IsSimulatingPhysics (.HitComponent (Collision|BreakHitResult _outhit)) "None")
            (Physics|AddImpulseatLocation (.HitComponent (Collision|BreakHitResult _outhit)) (* (Variables|Default|GetGunDirection) 2e+05) (.ImpactPoint (Collision|BreakHitResult _outhit)) "None")))))
    (elif (> (Variables|Default|GetAmmoCount) 0)
      (Game|SpawnActorfromClass "/Game/FirstPersonBP/Blueprints/FirstPersonProjectile.FirstPersonProjectile_C" (Math|Transform|MakeTransform (Transformation|GetWorldLocation (Variables|Default|GetBarrel_RefPoint)) (Transformation|GetWorldRotation (Variables|/Game/MyContent/Blueprints/Characters/MasterCharacter.MasterCharacter_C|GetFollowCamera (Variables|Default|GetGunOwner))) "1,1,1") "AlwaysSpawn" 0 0)
      (CallFunction|ThreatTrace (Variables|Default|GetThreatLevel))
      (Math|Integer|DecrementInt (Variables|Default|GetAmmoCount)))))

(fn ThreatTrace
  (params (InputPin :type Float%20%28single-precision%29))
  (bind _barrel_refpoint (Variables|Default|GetBarrel_RefPoint))
  (bind _returnvalue (Transformation|GetWorldLocation _barrel_refpoint))
  (bind _asarmed_combat_character (Utilities|Casting|CastToArmedCombatCharacter (Actor|GetParentActor)))
  (bind _outhit (Collision|SphereTraceByChannel _returnvalue (+ _returnvalue (* (Math|Vector|GetForwardVector (Transformation|GetWorldRotation (Variables|/Game/MyContent/Blueprints/Characters/MasterCharacter.MasterCharacter_C|GetFollowCamera _asarmed_combat_character))) (Variables|Default|GetRange))) InputPin "TraceTypeQuery2" false (Utilities|Array|MakeArray 0) "ForDuration" true "(R=0.009268,G=0.021773,B=1.000000,A=1.000000)" "(R=0.000000,G=0.795357,B=1.000000,A=1.000000)"))
  (if (.bblockinghit _outhit)
    (bind _asarmed_combat_character_2 (Utilities|Casting|CastToArmedCombatCharacter (.hitactor _outhit)))
    (Default|Threatened _asarmed_combat_character_2)))

(fn Reload
  (Variables|Default|SetBulletDifference (- (Variables|Default|GetClipSize) (Variables|Default|GetAmmoCount)))
  (if (>= (Variables|Default|GetAmmoMax) (Variables|Default|GetBulletDifference))
    (Variables|Default|SetAmmoCount (Variables|Default|GetClipSize))
    (Variables|Default|SetAmmoMax (- (Variables|Default|GetAmmoMax) (Variables|Default|GetBulletDifference)))
    (else
      (Variables|Default|SetAmmoCount (+ (Variables|Default|GetAmmoCount) (Variables|Default|GetAmmoMax)))
      (Variables|Default|SetAmmoMax 0))))